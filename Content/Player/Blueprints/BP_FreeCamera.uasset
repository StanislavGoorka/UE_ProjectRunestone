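; BP_FreeCamera is the player's free camera actor, a camera and spring arm that the view can switch to from a locked camera.
; Switching to free copies the given transform, FOV and arm length, then blends the controller's view target to this actor.
; Switching to locked messages the controller with the current arm length and resets the camera's relative location.
; Mouse wheel events step the arm length to zoom within passed-in limits.
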(event `self.ReceiveBeginPlay`
  (set `self.PlayerCharacterREF` (`GameplayStatics.GetPlayerCharacter` 0))
  (bind _output_get (set `self.PlayerControllerREF` (`PlayerState.GetPlayerController` (`GameplayStatics.GetPlayerState` 0))))
  (`self.EnableInput` _output_get))

(event `/Game/Player/BlueprintInterfaces/BPI_OnCameraUnlocked.OnCameraChangeToFree`
  (params (`Camera Transform` :type "Transform Structure") (`Camera FOV` :type "Float (double-precision)") (`Spring Arm Length` :type "Float (double-precision)"))
  (bind _springarm (`self.SpringArm`))
  (set `SpringArmComponent.TargetArmLength` `Spring Arm Length` _springarm)
  (`SceneComponent.K2_SetWorldTransform` _springarm `Camera Transform` false false)
  (`CameraComponent.SetFieldOfView` (`self.FreeCamera`) `Camera FOV`)
  (`PlayerController.SetViewTargetWithBlend` (`self.PlayerControllerREF`) (`ActorComponent.GetOwner` (`self.FreeCamera`)) 0.0 "VTBlend_Linear" 0.0 true))

(event `/Game/Player/BlueprintInterfaces/BPI_OnCameraUnlocked.OnCameraChangeToLocked`
  (params (`Spring Arm Length` :type "Float (double-precision)"))
  (message `/Game/Player/BlueprintInterfaces/BPI_OnCameraUnlocked.OnCameraChangeToLocked` (`self.PlayerControllerREF`) (`SpringArmComponent.TargetArmLength` (`self.SpringArm`)))
  (`SceneComponent.K2_SetRelativeLocation` (`self.FreeCamera`) (0.0 0.0 0.0) false false))

(event `/Game/Player/BlueprintInterfaces/BPI_OnCameraUnlocked.OnMouseWheelUp`
  (params (MinCameraOffset :type "Float (double-precision)") (MaxCameraOffset :type "Float (double-precision)") (CameraOffsetStep :type "Float (double-precision)"))
  (bind _springarm (`self.SpringArm`))
  (bind _targetarmlength (`SpringArmComponent.TargetArmLength` _springarm))
  (if (>= _targetarmlength MinCameraOffset)
    (set `SpringArmComponent.TargetArmLength` (- _targetarmlength CameraOffsetStep) _springarm)))

(event `/Game/Player/BlueprintInterfaces/BPI_OnCameraUnlocked.OnMouseWheelDown`
  (params (MinCameraOffset :type "Float (double-precision)") (MaxCameraOffset :type "Float (double-precision)") (CameraOffsetStep :type "Float (double-precision)"))
  (bind _springarm (`self.SpringArm`))
  (if (>= MaxCameraOffset (`SpringArmComponent.TargetArmLength` (`self.SpringArm`)))
    (set `SpringArmComponent.TargetArmLength` (+ (`SpringArmComponent.TargetArmLength` _springarm) CameraOffsetStep) _springarm)))

(fn `UserConstructionScript`)