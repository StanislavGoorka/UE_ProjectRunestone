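; Enemy spawner that creates a single BPC_Enemy after a delay each time its OnEnemySpawn event runs.
; BeginPlay reads the delay from the DefaultSpawnTime row of DT_Float, printing an error and keeping the variable's default if the row is missing.
; The enemy spawns at the Capsule's world transform and receives the calling event's Runestone reference through OnEnemySpawnMessage.
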(event `self.ReceiveBeginPlay`
  (bind _returnvalue (`|GetDataTableRow` "/Game/Data/DT_Float.DT_Float" "DefaultSpawnTime")
    (:`then`
      (set `self.SpawnTime` (`.Value_2_782D6C434D87971D775709941DF12983` (break `/Game/Data/DataStructures/S_Float` _returnvalue))))
    (:`RowNotFound`
      (`KismetSystemLibrary.PrintString` "Cannot find DefaultSpawnTime in DT_Float. Throwing default." true true (struct :`R` 1.0 :`A` 1.0) 5.0))))

(event `/Game/NPC/BlueprintInterfaces/BPI_OnEnemySpawn.OnEnemySpawn`
  (params (RunestoneREF :type "/Game/GameFlow/Blueprints/BP_Runestone Object Reference"))
  (`KismetSystemLibrary.Delay` (`self.SpawnTime`))
  (bind _returnvalue (`|SpawnActorFromClass` "/Game/NPC/Blueprints/BPC_Enemy.BPC_Enemy_C" (`SceneComponent.K2_GetComponentToWorld` (`self.Capsule`)) "Undefined" "MultiplyWithRoot" null null))
  (message `/Game/NPC/BlueprintInterfaces/BPI_OnEnemySpawn.OnEnemySpawn` _returnvalue RunestoneREF))

(fn `UserConstructionScript`)