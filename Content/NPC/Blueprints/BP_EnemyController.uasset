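; BP_EnemyController drives enemy spawning in the level around the BP_Runestone actor.
; On BeginPlay it caches the runestone and all BP_EnemySpawner actors, then binds and immediately calls BeginSpawning, or prints a red warning if no runestone is found.
; BeginSpawning starts a looping one-second timer that sends OnEnemySpawnMessage to a random spawner, passing the runestone reference.
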(event `self.ReceiveBeginPlay`
  (bind _returnvalue (`GameplayStatics.GetActorOfClass` "/Game/GameFlow/Blueprints/BP_Runestone.BP_Runestone_C"))
  (`/Engine/EditorBlueprintResources/StandardMacros.IsValid` _returnvalue
    (:`Is Valid`
      (set `self.RunestoneREF` _returnvalue)
      (bind _outactors (`GameplayStatics.GetAllActorsOfClass` "/Game/NPC/Blueprints/BP_EnemySpawner.BP_EnemySpawner_C"))
      (set `self.EnemySpawnersREF` _outactors)
      (add `self.BeginSpawning` (delegate `BeginSpawning_Event`))
      (`self.BeginSpawning`))
    (:`Is Not Valid`
      (`KismetSystemLibrary.PrintString` "WARNING: Couldn't find valid object of class BP_Runestone" true true (struct :`R` 1.0 :`A` 1.0) 5.0))))

(event `BeginSpawning_Event`
  (`KismetSystemLibrary.K2_SetTimerDelegate` (delegate `TimerTick`) 1.0 true))

(event `TimerTick`
  (message `/Game/NPC/BlueprintInterfaces/BPI_OnEnemySpawn.OnEnemySpawn` (`KismetArrayLibrary.Array_Random` (`self.EnemySpawnersREF`)) (`self.RunestoneREF`)))

(fn `UserConstructionScript`)